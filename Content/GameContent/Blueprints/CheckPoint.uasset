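; Checkpoint actor that saves the player's respawn point when anything overlaps its CheckPointAOE volume.
; It sets the first-person character's SpawnTransform to just above its Platform, using the platform's rotation, and clears LastCheckpointTransform on the DataManager game instance.
; It then loads or creates the SavedData save object, stores the transform as LastCheckpoint, saves it and prints the result for debugging.
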(event OnComponentBeginOverlap(CheckPointAOE)
  (params (OverlappedComponent :type Primitive%20Component%20Object%20Reference) (OtherActor :type Actor%20Object%20Reference) (OtherComp :type Primitive%20Component%20Object%20Reference) (OtherBodyIndex :type Integer) (bFromSweep :type Boolean) (SweepResult :type Hit%20Result%20Structure%20%28by%20ref%29))
  (bind _savename (Variables|Default|Getsavename))
  (bind _platform (Variables|Default|GetPlatform))
  (bind _returnvalue (Transformation|GetWorldTransform _platform))
  (bind (_location _rotation) (Math|Transform|BreakTransform _returnvalue))
  (bind _asfirst_person_character (Utilities|Casting|CastToFirstPersonCharacter (Game|GetPlayerCharacter 0)))
  (bind _output_get (Variables|/Game/FirstPersonBP/Blueprints/FirstPersonCharacter.FirstPersonCharacter_C|SetspawnTransform _asfirst_person_character (Math|Transform|MakeTransform (+ _location "0, 0,128.000000") _rotation)))
  (bind _asdata_manager (Utilities|Casting|CastToDataManager (Game|GetGameInstance)))
  (Variables|/Game/GameContent/Blueprints/TextSystem/DataManager.DataManager_C|SetlastCheckpointTransform _asdata_manager "")
  (bind _returnvalue_2 (SaveGame|DoesSaveGameExist (Variables|Default|Getsavename)))
  (if _returnvalue_2
    (bind _returnvalue_3 (SaveGame|LoadGamefromSlot (Variables|Default|Getsavename)))
    (Variables|Default|Setsub%20class _returnvalue_3)
    (bind _assaved_data (Utilities|Casting|CastToSavedData (Variables|Default|Getsub%20class)))
    (bind _output_get_2 (Variables|/Game/SavedData.SavedData_C|SetlastCheckpoint _assaved_data _output_get))
    (bind _returnvalue_4 (SaveGame|SaveGametoSlot (Variables|Default|Getsub%20class) _savename))
    (Development|PrintString (Utilities|String|ToString(Boolean) _returnvalue_4))
    (Development|PrintString (Utilities|String|ToString(Transform) _output_get_2))
    (else
      (bind _returnvalue_5 (SaveGame|CreateSaveGameObject "/Game/SavedData.SavedData_C"))
      (Variables|Default|Setsub%20class _returnvalue_5)
      (bind _assaved_data_2 (Utilities|Casting|CastToSavedData (Variables|Default|Getsub%20class)))
      (bind _output_get_3 (Variables|/Game/SavedData.SavedData_C|SetlastCheckpoint _assaved_data_2 _output_get))
      (bind _returnvalue_6 (SaveGame|SaveGametoSlot (Variables|Default|Getsub%20class) _savename))
      (Development|PrintString (Utilities|String|ToString(Boolean) _returnvalue_6))
      (Development|PrintString (Utilities|String|ToString(Transform) _output_get_3)))))

(fn ConstructionScript)