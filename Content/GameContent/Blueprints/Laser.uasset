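; Laser hazard actor that destroys the first-person character when it overlaps the laser's collision component.
; Every tick, a long Visibility line trace runs forward from the Laser component, with per-frame debug drawing on.
; On a hit, the beam's X scale is set from the hit distance, so it stretches to the first blocking surface.
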(event OnComponentBeginOverlap(LaserCol)
  (params (OverlappedComponent :type Primitive%20Component%20Object%20Reference) (OtherActor :type Actor%20Object%20Reference) (OtherComp :type Primitive%20Component%20Object%20Reference) (OtherBodyIndex :type Integer) (bFromSweep :type Boolean) (SweepResult :type Hit%20Result%20Structure%20%28by%20ref%29))
  (bind _asfirst_person_character (Utilities|Casting|CastToFirstPersonCharacter OtherActor))
  (Actor|DestroyActor _asfirst_person_character))

(event EventBeginPlay)

(event Collision|EventActorBeginOverlap
  (params (OtherActor :type Actor%20Object%20Reference)))

(event EventTick
  (params (DeltaSeconds :type Float%20%28single-precision%29))
  (CallFunction|LaserScale))

(fn ConstructionScript)

(fn LaserScale
  (bind _laser (Variables|Default|GetLaser))
  (bind _returnvalue (Transformation|GetWorldLocation _laser))
  (bind (_outhit _returnvalue_2) (Collision|LineTraceByChannel _returnvalue (+ _returnvalue (* (Math|Vector|GetForwardVector _laser) 888888.0)) "TraceTypeQuery1" false 0 "ForOneFrame"))
  (if _returnvalue_2
    (Transformation|SetWorldScale3D (Variables|Default|GetLaser) (Math|Vector|MakeVector (/ (Math|Vector|VectorLength (- (.Location (Collision|BreakHitResult _outhit)) (.TraceStart (Collision|BreakHitResult _outhit)))) 1e+02) 0.6 0.3))))