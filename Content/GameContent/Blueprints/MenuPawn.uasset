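; MenuPawn is a pawn that presents the end screen and handles its keyboard input.
; On BeginPlay it adds an EndScreenHud widget to the viewport, then runs a timeline whose curve drives the color and opacity of that widget's white fade element.
; Escape quits the game, and Enter opens the Gemu level.
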(event Collision|EventActorBeginOverlap
  (params (OtherActor :type Actor%20Object%20Reference)))

(event EventBeginPlay
  (bind _returnvalue (UserInterface|CreateWidget "/Game/GameContent/Blueprints/EndScreenHud.EndScreenHud_C"))
  (UserInterface|Viewport|AddtoViewport _returnvalue 0)
  (bind _foundwidgets (Widget|GetAllWidgetsOfClass "/Game/GameContent/Blueprints/EndScreenHud.EndScreenHud_C" true))
  (bind _endscreenwhitecurve (Timeline|WhiteFadeTimeline Play)
    (:Update
      (Appearance|SetColorandOpacity (Variables|/Game/GameContent/Blueprints/EndScreenHud.EndScreenHud_C|GetEndScreenWhiteFade (Utilities|Array|Get(acopy) _foundwidgets)) _endscreenwhitecurve :!class /Script/UMG.Image))))

(event EventTick
  (params (DeltaSeconds :type Float%20%28single-precision%29)))

(event Input|KeyboardEvents|Escape
  (params (Key :type Key%20Structure))
  (:Pressed
    (Game|QuitGame 0 "Quit")))

(event Input|KeyboardEvents|Enter
  (params (Key :type Key%20Structure))
  (:Pressed
    (Game|OpenLevel(byName) "Gemu")))

(fn ConstructionScript)