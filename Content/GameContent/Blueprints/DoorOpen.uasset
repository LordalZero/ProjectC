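; A two-piece sliding door that opens when the first-person character enters its trigger and closes when they leave.
; BeginPlay caches each piece's start position, takes end positions from marker components and sets both timelines' play rate.
; Two timelines lerp the upper and lower pieces between those points, reversing on exit.
; The indicator material switches on any overlap, before the character check; the IsActive branch and SetLocations are empty.
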(event OnComponentBeginOverlap(PlayerTouch)
  (params (OverlappedComponent :type Primitive%20Component%20Object%20Reference) (OtherActor :type Actor%20Object%20Reference) (OtherComp :type Primitive%20Component%20Object%20Reference) (OtherBodyIndex :type Integer) (bFromSweep :type Boolean) (SweepResult :type Hit%20Result%20Structure%20%28by%20ref%29))
  (Rendering|Material|SetMaterial (Variables|Default|GetDoorIndicator) 2 "/Game/GameContent/Materials/OrangeGlow.OrangeGlow")
  (Utilities|Casting|CastToFirstPersonCharacter OtherActor)
  (Utilities|FlowControl|Sequence
    (:then_0
      (bind _upperpiecemovement (Timeline|PieceUp Play)
        (:Update
          (Transformation|SetWorldLocation (Variables|Default|GetUpperPiece) (Math|Vector|Lerp(Vector) (Variables|Default|GetUpperPieceStart) (Variables|Default|GetUpperPieceEnd) _upperpiecemovement) false false))))
    (:then_1
      (bind _lowerpiecemovement (Timeline|DownPiece Play)
        (:Update
          (Transformation|SetWorldLocation (Variables|Default|GetLowerPiece) (Math|Vector|Lerp(Vector) (Variables|Default|GetLowerPieceStart) (Variables|Default|GetLowerPieceEnd) _lowerpiecemovement) false false))))))

(event OnComponentEndOverlap(PlayerTouch)
  (params (OverlappedComponent :type Primitive%20Component%20Object%20Reference) (OtherActor :type Actor%20Object%20Reference) (OtherComp :type Primitive%20Component%20Object%20Reference) (OtherBodyIndex :type Integer))
  (Rendering|Material|SetMaterial (Variables|Default|GetDoorIndicator) 2 "/Game/GameContent/Materials/ChromaticBlackFloor.ChromaticBlackFloor")
  (Utilities|Casting|CastToFirstPersonCharacter OtherActor)
  (Utilities|FlowControl|Sequence
    (:then_0
      (bind _upperpiecemovement (Timeline|PieceUp Reverse)
        (:Update
          (Transformation|SetWorldLocation (Variables|Default|GetUpperPiece) (Math|Vector|Lerp(Vector) (Variables|Default|GetUpperPieceStart) (Variables|Default|GetUpperPieceEnd) _upperpiecemovement) false false))))
    (:then_1
      (bind _lowerpiecemovement (Timeline|DownPiece Reverse)
        (:Update
          (Transformation|SetWorldLocation (Variables|Default|GetLowerPiece) (Math|Vector|Lerp(Vector) (Variables|Default|GetLowerPieceStart) (Variables|Default|GetLowerPieceEnd) _lowerpiecemovement) false false))))))

(event EventBeginPlay
  (Variables|Default|SetUpperPieceStart (Transformation|GetWorldLocation (Variables|Default|GetUpperPiece)))
  (Variables|Default|SetLowerPieceStart (Transformation|GetWorldLocation (Variables|Default|GetLowerPiece)))
  (Variables|Default|SetUpperPieceEnd (Transformation|GetWorldLocation (Variables|Default|GetUpperPieceCoor)))
  (Variables|Default|SetLowerPieceEnd (Transformation|GetWorldLocation (Variables|Default|GetLowerPieceCoor)))
  (Components|Timeline|SetPlayRate (Variables|Default|GetPieceUp) (Variables|Default|GetPlayRate))
  (Components|Timeline|SetPlayRate (Variables|Default|GetDownPiece) (Variables|Default|GetPlayRate))
  (if (Variables|Default|GetIsActive)
    _))

(fn ConstructionScript)

(fn SetLocations)