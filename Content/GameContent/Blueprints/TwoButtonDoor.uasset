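; Two-switch door that opens only while both touch triggers are occupied and closes when either is empty.
; Each trigger keeps an overlap count, printed for debugging, which Tick converts into switch flags.
; When both flags are set, two timelines play to lerp the upper and lower pieces from their start positions to marker component locations cached at BeginPlay; otherwise the timelines reverse.
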(event OnComponentBeginOverlap(PlayerTouch1)
  (params (OverlappedComponent :type Primitive%20Component%20Object%20Reference) (OtherActor :type Actor%20Object%20Reference) (OtherComp :type Primitive%20Component%20Object%20Reference) (OtherBodyIndex :type Integer) (bFromSweep :type Boolean) (SweepResult :type Hit%20Result%20Structure%20%28by%20ref%29))
  (bind _output_get (Variables|Default|SetoverlappingActortouch1 (+ (Variables|Default|GetoverlappingActortouch1) 1)))
  (Development|PrintString (Utilities|String|ToString(Integer) _output_get)))

(event OnComponentEndOverlap(PlayerTouch1)
  (params (OverlappedComponent :type Primitive%20Component%20Object%20Reference) (OtherActor :type Actor%20Object%20Reference) (OtherComp :type Primitive%20Component%20Object%20Reference) (OtherBodyIndex :type Integer))
  (bind _output_get (Variables|Default|SetoverlappingActortouch1 (- (Variables|Default|GetoverlappingActortouch1) 1)))
  (Development|PrintString (Utilities|String|ToString(Integer) _output_get)))

(event OnComponentBeginOverlap(PlayerTouch2)
  (params (OverlappedComponent :type Primitive%20Component%20Object%20Reference) (OtherActor :type Actor%20Object%20Reference) (OtherComp :type Primitive%20Component%20Object%20Reference) (OtherBodyIndex :type Integer) (bFromSweep :type Boolean) (SweepResult :type Hit%20Result%20Structure%20%28by%20ref%29))
  (bind _output_get (Variables|Default|SetoverlappingActortouch2 (+ (Variables|Default|GetoverlappingActortouch2) 1)))
  (Development|PrintString (Utilities|String|ToString(Integer) _output_get) true true "(R=1.000000,G=0.000000,B=0.184016,A=1.000000)"))

(event OnComponentEndOverlap(PlayerTouch2)
  (params (OverlappedComponent :type Primitive%20Component%20Object%20Reference) (OtherActor :type Actor%20Object%20Reference) (OtherComp :type Primitive%20Component%20Object%20Reference) (OtherBodyIndex :type Integer))
  (bind _output_get (Variables|Default|SetoverlappingActortouch2 (- (Variables|Default|GetoverlappingActortouch2) 1)))
  (Development|PrintString (Utilities|String|ToString(Integer) _output_get) true true "(R=1.000000,G=0.000000,B=0.184016,A=1.000000)"))

(event EventBeginPlay
  (Variables|Default|SetUpperPieceStart (Transformation|GetWorldLocation (Variables|Default|GetUpperPiece)))
  (Variables|Default|SetLowerPieceStart (Transformation|GetWorldLocation (Variables|Default|GetLowerPiece)))
  (Variables|Default|SetUpperPieceEnd (Transformation|GetWorldLocation (Variables|Default|GetUpperPieceCoor)))
  (Variables|Default|SetLowerPieceEnd (Transformation|GetWorldLocation (Variables|Default|GetLowerPieceCoor)))
  (Components|Timeline|SetPlayRate (Variables|Default|GetPieceUp) (Variables|Default|GetPlayRate))
  (Components|Timeline|SetPlayRate (Variables|Default|GetDownPiece) (Variables|Default|GetPlayRate)))

(event EventTick
  (params (DeltaSeconds :type Float%20%28single-precision%29))
  (Utilities|FlowControl|Sequence
    (:then_0
      (if (> (Variables|Default|GetoverlappingActortouch1) 0)
        (Variables|Default|Setswitch1On true)
        (else
          (Variables|Default|Setswitch1On false))))
    (:then_1
      (if (> (Variables|Default|GetoverlappingActortouch2) 0)
        (Variables|Default|Setswitch2On true)
        (else
          (Variables|Default|Setswitch2On false)))))
  (if (and (Variables|Default|Getswitch1On) (Variables|Default|Getswitch2On))
    (Utilities|FlowControl|Sequence
      (:then_0
        (bind _upperpiecemovement (Timeline|PieceUp Play)
          (:Update
            (Transformation|SetWorldLocation (Variables|Default|GetUpperPiece) (Math|Vector|Lerp(Vector) (Variables|Default|GetUpperPieceStart) (Variables|Default|GetUpperPieceEnd) _upperpiecemovement) false false))))
      (:then_1
        (bind _lowerpiecemovement (Timeline|DownPiece Play)
          (:Update
            (Transformation|SetWorldLocation (Variables|Default|GetLowerPiece) (Math|Vector|Lerp(Vector) (Variables|Default|GetLowerPieceStart) (Variables|Default|GetLowerPieceEnd) _lowerpiecemovement) false false)))))
    (else
      (Utilities|FlowControl|Sequence
        (:then_0
          (Timeline|PieceUp Reverse))
        (:then_1
          (Timeline|DownPiece Reverse))))))

(fn ConstructionScript)

(fn SetLocations)