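; Laser hazard actor that sends the player back to the last checkpoint and destroys translocator devices that cross its beam.
; Every Tick it line-traces between two cube components on a custom trace channel, with the one-frame debug line drawn.
; On a hit it loads the SavedData save slot, then passes LastCheckpoint to the character's RespawnPlayer or destroys the hit TranslocatorDevice.
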(event EventTick
  (params (DeltaSeconds :type Float%20%28single-precision%29))
  (bind (_outhit _returnvalue) (Collision|LineTraceByChannel (Transformation|GetWorldLocation (Variables|Default|GetCube_1)) (Transformation|GetWorldLocation (Variables|Default|GetCube_2)) "TraceTypeQuery3" false 0 "ForOneFrame"))
  (if _returnvalue
    (Utilities|FlowControl|Sequence
      (:then_0
        (bind _returnvalue_2 (SaveGame|LoadGamefromSlot "slot"))
        (bind _assaved_data (Utilities|Casting|CastToSavedData _returnvalue_2)))
      (:then_1
        (bind _asfirst_person_character (Utilities|Casting|CastToFirstPersonCharacter (.hitactor _outhit)))
        (Default|RespawnPlayer _asfirst_person_character (Variables|/Game/GameContent/SavedData.SavedData_C|GetlastCheckpoint _assaved_data)))
      (:then_2
        (bind _astranslocator_device (Utilities|Casting|CastToTranslocatorDevice (.hitactor _outhit)))
        (Actor|DestroyActor (.hitactor _outhit))))))

(fn ConstructionScript)