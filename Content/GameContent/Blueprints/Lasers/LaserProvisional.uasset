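; Provisional laser hazard actor that, while IsActive, resets the player or the thrown translocator device when either overlaps the beam.
; Tick sets the Lazer component's visibility to match IsActive, and the overlap event checks the same flag.
; An overlapping FirstPersonCharacter respawns at the LastCheckpoint loaded from the save slot.
; An overlapping TranslocatorDevice spawns a return animation, clears the player's Thrown state and is destroyed.
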(event OnComponentBeginOverlap(lazer)
  (params (OverlappedComponent :type Primitive%20Component%20Object%20Reference) (OtherActor :type Actor%20Object%20Reference) (OtherComp :type Primitive%20Component%20Object%20Reference) (OtherBodyIndex :type Integer) (bFromSweep :type Boolean) (SweepResult :type Hit%20Result%20Structure%20%28by%20ref%29))
  (if (Variables|Default|GetIs%20Active)
    (Utilities|FlowControl|Sequence
      (:then_0
        (bind _returnvalue (SaveGame|LoadGamefromSlot "slot"))
        (bind _assaved_data (Utilities|Casting|CastToSavedData _returnvalue)))
      (:then_1
        (bind _asfirst_person_character (Utilities|Casting|CastToFirstPersonCharacter OtherActor))
        (Default|RespawnPlayer _asfirst_person_character (Variables|/Game/GameContent/SavedData.SavedData_C|GetlastCheckpoint _assaved_data)))
      (:then_2
        (bind _astranslocator_device (Utilities|Casting|CastToTranslocatorDevice OtherActor))
        (Game|SpawnActorfromClass "/Game/GameContent/Blueprints/TD_ReturnAnim.TD_ReturnAnim_C" (Math|Conversions|ToTransform(Vector) (Transformation|GetActorLocation _astranslocator_device)) "AdjustIfPossibleButAlwaysSpawn" 0 0)
        (bind _asfirst_person_character_2 (Utilities|Casting|CastToFirstPersonCharacter (Game|GetPlayerCharacter 0)))
        (Variables|/Game/FirstPersonBP/Blueprints/FirstPersonCharacter.FirstPersonCharacter_C|Setthrown _asfirst_person_character_2 0)
        (Actor|DestroyActor _astranslocator_device)))))

(event EventTick
  (params (DeltaSeconds :type Float%20%28single-precision%29))
  (if (Variables|Default|GetIs%20Active)
    (Rendering|SetVisibility (Variables|Default|Getlazer) true false)
    (else
      (Rendering|SetVisibility (Variables|Default|Getlazer) false false))))

(fn ConstructionScript)