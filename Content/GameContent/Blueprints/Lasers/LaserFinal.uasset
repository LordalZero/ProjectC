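; Laser barrier that sends the player back to the last saved checkpoint on hit and destroys TranslocatorDevices crossing it.
; While IsActive, Tick stretches the beam between SideA and SideB and resets the player's Thrown value every frame; otherwise the beam scales to zero.
; OtherLines runs eight extra line traces between marker pairs to catch the devices.
; Debug leftovers include a U key that destroys the first device and a "Hello" print.
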(event OnComponentHit(LaserLine)
  (params (HitComponent :type Primitive%20Component%20Object%20Reference) (OtherActor :type Actor%20Object%20Reference) (OtherComp :type Primitive%20Component%20Object%20Reference) (NormalImpulse :type Vector :default "0, 0, 0") (Hit :type Hit%20Result%20Structure%20%28by%20ref%29))
  (Utilities|FlowControl|Sequence
    (:then_0
      (bind _returnvalue (SaveGame|LoadGamefromSlot "slot"))
      (bind _assaved_data (Utilities|Casting|CastToSavedData _returnvalue)))
    (:then_1
      (bind _asfirst_person_character (Utilities|Casting|CastToFirstPersonCharacter OtherActor))
      (Default|RespawnPlayer _asfirst_person_character (Variables|/Game/GameContent/SavedData.SavedData_C|GetlastCheckpoint _assaved_data)))
    (:then_2
      (Utilities|Casting|CastToTranslocatorDevice OtherActor)
      (Development|PrintString "Hello"))))

(event EventBeginPlay)

(event Collision|EventActorBeginOverlap
  (params (OtherActor :type Actor%20Object%20Reference)))

(event EventTick
  (params (DeltaSeconds :type Float%20%28single-precision%29))
  (if (Variables|Default|GetIsActive)
    (CallFunction|LaserScale)
    (else
      (Transformation|SetWorldScale3D (Variables|Default|GetLaser) "0, 0, 0"))))

(event Input|KeyboardEvents|U
  (params (Key :type Key%20Structure))
  (:Pressed
    (bind _outactors (Actor|GetAllActorsOfClass "/Game/GameContent/Blueprints/TranslocatorDevice.TranslocatorDevice_C"))
    (Actor|DestroyActor (Utilities|Array|Get(acopy) _outactors))))

(fn ConstructionScript)

(fn LaserScale
  (if (Variables|Default|GetIsActive)
    (Utilities|FlowControl|Sequence
      (:then_0
        (Collision|LineTraceByChannel (Transformation|GetWorldLocation (Variables|Default|GetSideA)) (Transformation|GetWorldLocation (Variables|Default|GetSideB)) "TraceTypeQuery3" false 0 "None")
        (Transformation|SetWorldScale3D (Variables|Default|GetLaser) (Math|Vector|MakeVector (/ (Math|Vector|VectorLength (- (Transformation|GetWorldLocation (Variables|Default|GetSideA)) (Transformation|GetWorldLocation (Variables|Default|GetSideB)))) 1e+02) 0.6 0.3)))
      (:then_1
        (CallFunction|OtherLines)))
    (bind _asfirst_person_character (Utilities|Casting|CastToFirstPersonCharacter (Game|GetPlayerCharacter 0)))
    (Variables|/Game/FirstPersonBP/Blueprints/FirstPersonCharacter.FirstPersonCharacter_C|Setthrown _asfirst_person_character 0)))

(fn OtherLines
  (Utilities|FlowControl|Sequence
    (:then_0
      (bind (_outhit _returnvalue) (Collision|LineTraceByChannel (Transformation|GetWorldLocation (Variables|Default|GetFirstLaserA)) (Transformation|GetWorldLocation (Variables|Default|GetFirstLaserB)) "TraceTypeQuery3" false 0 "None"))
      (if _returnvalue
        (Utilities|FlowControl|Sequence
          (:then_2
            (bind _astranslocator_device (Utilities|Casting|CastToTranslocatorDevice (.hitactor _outhit)))
            (Actor|DestroyActor (.hitactor _outhit))))))
    (:then_1
      (bind (_outhit_2 _returnvalue_2) (Collision|LineTraceByChannel (Transformation|GetWorldLocation (Variables|Default|GetSecondLaserA)) (Transformation|GetWorldLocation (Variables|Default|GetStaticMeshB)) "TraceTypeQuery3" false 0 "None"))
      (if _returnvalue_2
        (Utilities|FlowControl|Sequence
          (:then_2
            (bind _astranslocator_device_2 (Utilities|Casting|CastToTranslocatorDevice (.hitactor _outhit_2)))
            (Actor|DestroyActor (.hitactor _outhit_2))))))
    (:then_2
      (bind (_outhit_3 _returnvalue_3) (Collision|LineTraceByChannel (Transformation|GetWorldLocation (Variables|Default|GetThird%20LaserA)) (Transformation|GetWorldLocation (Variables|Default|GetThird%20LaserB)) "TraceTypeQuery3" false 0 "None"))
      (if _returnvalue_3
        (Utilities|FlowControl|Sequence
          (:then_2
            (bind _astranslocator_device_3 (Utilities|Casting|CastToTranslocatorDevice (.hitactor _outhit_3)))
            (Actor|DestroyActor (.hitactor _outhit_3))))))
    (:then_3
      (bind (_outhit_4 _returnvalue_4) (Collision|LineTraceByChannel (Transformation|GetWorldLocation (Variables|Default|GetFourthLaserA)) (Transformation|GetWorldLocation (Variables|Default|GetFourthLaserB)) "TraceTypeQuery3" false 0 "None"))
      (if _returnvalue_4
        (Utilities|FlowControl|Sequence
          (:then_2
            (bind _astranslocator_device_4 (Utilities|Casting|CastToTranslocatorDevice (.hitactor _outhit_4)))
            (Actor|DestroyActor (.hitactor _outhit_4))))))
    (:then_4
      (bind (_outhit_5 _returnvalue_5) (Collision|LineTraceByChannel (Transformation|GetWorldLocation (Variables|Default|GetSixth%20Lase%20A)) (Transformation|GetWorldLocation (Variables|Default|GetSixthLaser%20B)) "TraceTypeQuery3" false 0 "None"))
      (if _returnvalue_5
        (Utilities|FlowControl|Sequence
          (:then_2
            (bind _astranslocator_device_5 (Utilities|Casting|CastToTranslocatorDevice (.hitactor _outhit_5)))
            (Actor|DestroyActor (.hitactor _outhit_5))))))
    (:then_5
      (bind (_outhit_6 _returnvalue_6) (Collision|LineTraceByChannel (Transformation|GetWorldLocation (Variables|Default|GetFithLaserA)) (Transformation|GetWorldLocation (Variables|Default|GetFithLaserB)) "TraceTypeQuery3" false 0 "None"))
      (if _returnvalue_6
        (Utilities|FlowControl|Sequence
          (:then_2
            (bind _astranslocator_device_6 (Utilities|Casting|CastToTranslocatorDevice (.hitactor _outhit_6)))
            (Actor|DestroyActor (.hitactor _outhit_6))))))
    (:then_6
      (bind (_outhit_7 _returnvalue_7) (Collision|LineTraceByChannel (Transformation|GetWorldLocation (Variables|Default|GetEigth%20Laser%20A)) (Transformation|GetWorldLocation (Variables|Default|GetEigthLaserB)) "TraceTypeQuery3" false 0 "None"))
      (if _returnvalue_7
        (Utilities|FlowControl|Sequence
          (:then_2
            (bind _astranslocator_device_7 (Utilities|Casting|CastToTranslocatorDevice (.hitactor _outhit_7)))
            (Actor|DestroyActor (.hitactor _outhit_7))))))
    (:then_7
      (bind (_outhit_8 _returnvalue_8) (Collision|LineTraceByChannel (Transformation|GetWorldLocation (Variables|Default|GetSeventh%20Laser%20A)) (Transformation|GetWorldLocation (Variables|Default|GetSeventh%20Laser%20B)) "TraceTypeQuery3" false 0 "None"))
      (if _returnvalue_8
        (Utilities|FlowControl|Sequence
          (:then_2
            (bind _astranslocator_device_8 (Utilities|Casting|CastToTranslocatorDevice (.hitactor _outhit_8)))
            (Actor|DestroyActor (.hitactor _outhit_8))))))))