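; LaserSwitch is an interactable switch that temporarily deactivates every LaserProvisional in the level.
; Overlapping its trigger enables player input and leaving disables it, with the character cast running only afterwards, so it filters nothing.
; Interact sets IsActive false on all lasers, then sets it true again after Laseroffdelay.
; The Delay sits inside the first loop body rather than on its completion.
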(event OnComponentBeginOverlap(Trigger)
  (params (OverlappedComponent :type Primitive%20Component%20Object%20Reference) (OtherActor :type Actor%20Object%20Reference) (OtherComp :type Primitive%20Component%20Object%20Reference) (OtherBodyIndex :type Integer) (bFromSweep :type Boolean) (SweepResult :type Hit%20Result%20Structure%20%28by%20ref%29))
  (Input|EnableInput (Game|GetPlayerController 0))
  (Utilities|Casting|CastToFirstPersonCharacter OtherActor))

(event OnComponentEndOverlap(Trigger)
  (params (OverlappedComponent :type Primitive%20Component%20Object%20Reference) (OtherActor :type Actor%20Object%20Reference) (OtherComp :type Primitive%20Component%20Object%20Reference) (OtherBodyIndex :type Integer))
  (Input|DisableInput (Game|GetPlayerController 0))
  (Utilities|Casting|CastToFirstPersonCharacter OtherActor))

(event Input|ActionEvents|InputActionInteract
  (params (Key :type Key%20Structure))
  (:Pressed
    (bind _outactors (Actor|GetAllActorsOfClass "/Game/GameContent/Blueprints/Lasers/LaserProvisional.LaserProvisional_C"))
    (for _array_element _outactors
      (Variables|/Game/GameContent/Blueprints/Lasers/LaserProvisional.LaserProvisional_C|SetIs%20Active _array_element false)
      (Utilities|FlowControl|Delay (Variables|Default|Getlaseroffdelay))
      (bind _outactors_2 (Actor|GetAllActorsOfClass "/Game/GameContent/Blueprints/Lasers/LaserProvisional.LaserProvisional_C"))
      (for _array_element_2 _outactors_2
        (Variables|/Game/GameContent/Blueprints/Lasers/LaserProvisional.LaserProvisional_C|SetIs%20Active _array_element_2 true)))))

(fn ConstructionScript)