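; Trigger actor that shows a sequence of subtitle lines with voice audio once the first-person player overlaps its collider.
; Tick picks English or Spanish text and sound arrays from the DataManager game instance's language setting.
; A DoOnce gate steps through lines, creating a widget for each and resetting after the clip's duration plus a delay.
; Voice volume comes from the save game; only the English branch destroys the actor when finished.
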(event OnComponentBeginOverlap(Collider)
  (params (OverlappedComponent :type Primitive%20Component%20Object%20Reference) (OtherActor :type Actor%20Object%20Reference) (OtherComp :type Primitive%20Component%20Object%20Reference) (OtherBodyIndex :type Integer) (bFromSweep :type Boolean) (SweepResult :type Hit%20Result%20Structure%20%28by%20ref%29))
  (Utilities|Casting|CastToFirstPersonCharacter (Game|GetPlayerCharacter 0))
  (Variables|Default|SetstartDisplaytxt true))

(event EventTick
  (params (DeltaSeconds :type Float%20%28single-precision%29))
  (bind _asdata_manager (Utilities|Casting|CastToDataManager (Game|GetGameInstance)))
  (switch int (Variables|/Game/GameContent/Blueprints/TextSystem/DataManager.DataManager_C|GetLanguages _asdata_manager)
    (:Default
      (if (Variables|Default|GetstartDisplaytxt) :!label _label
        (Utilities|FlowControl|DoOnce false :!label _label_2
          (:Completed
            (bind _returnvalue (UserInterface|CreateWidget "/Game/GameContent/Blueprints/TextSystem/TextSystemTest.TextSystemTest_C"))
            (Variables|/Game/GameContent/Blueprints/TextSystem/TextSystemTest.TextSystemTest_C|SettxtDisplay _returnvalue (Utilities|Array|Get(acopy) (Variables|Default|GetDisplayedText%28Ensglish%29) (Variables|Default|GetcurrentDisplay)))
            (bind _output_get (Variables|Default|SetsoundChose (Utilities|Array|Get(acopy) (Variables|Default|GetDisplayedSound%28English%29) (Variables|Default|GetcurrentDisplay))))
            (CallFunction|GetVoiceVol _output_get)
            (UserInterface|Viewport|AddtoViewport _returnvalue 0)
            (if (>= (Variables|Default|GetcurrentDisplay) (Utilities|Array|Length (Variables|Default|GetDisplayedText%28Ensglish%29)))
              (Widget|RemovefromParent _returnvalue)
              (Actor|DestroyActor)
              (else
                (Variables|Default|SetcurrentDisplay (+ (Variables|Default|GetcurrentDisplay) (Variables|Default|GetintIncrease)))
                (Utilities|FlowControl|Delay (+ (Variables|/Script/Engine.SoundBase|GetDuration (Variables|Default|GetsoundChose)) (Variables|Default|GetdelayBetweenLines)))
                (Widget|RemovefromParent _returnvalue)
                (goto _label_2 Reset)))))))
    (:0
      (goto _label))
    (:1
      (if (Variables|Default|GetstartDisplaytxt)
        (Utilities|FlowControl|DoOnce false :!label _label_3
          (:Completed
            (bind _returnvalue_2 (UserInterface|CreateWidget "/Game/GameContent/Blueprints/TextSystem/TextSystemTest.TextSystemTest_C"))
            (Variables|/Game/GameContent/Blueprints/TextSystem/TextSystemTest.TextSystemTest_C|SettxtDisplay _returnvalue_2 (Utilities|Array|Get(acopy) (Variables|Default|GetDisplayedText%28Spanish%29) (Variables|Default|GetcurrentDisplay)))
            (bind _output_get_2 (Variables|Default|SetsoundChose (Utilities|Array|Get(acopy) (Variables|Default|GetDisplayedSound%28Spanish%29) (Variables|Default|GetcurrentDisplay))))
            (UserInterface|Viewport|AddtoViewport _returnvalue_2 0)
            (CallFunction|GetVoiceVol _output_get_2)
            (if (>= (Variables|Default|GetcurrentDisplay) (Utilities|Array|Length (Variables|Default|GetDisplayedText%28Spanish%29)))
              (Widget|RemovefromParent _returnvalue_2)
              (else
                (Variables|Default|SetcurrentDisplay (+ (Variables|Default|GetcurrentDisplay) (Variables|Default|GetintIncrease)))
                (Utilities|FlowControl|Delay (+ (Variables|/Script/Engine.SoundBase|GetDuration (Variables|Default|GetsoundChose)) (Variables|Default|GetdelayBetweenLines)))
                (Widget|RemovefromParent _returnvalue_2)
                (goto _label_3 Reset)))))))))

(fn ConstructionScript)

(fn GetVoiceVol
  (params (Voice :type Sound%20Base%20Object%20Reference))
  (bind _returnvalue (SaveGame|LoadGamefromSlot (Variables|Default|Getsavename)))
  (bind _assaved_data (Utilities|Casting|CastToSavedData _returnvalue))
  (Audio|PlaySound2D Voice (Variables|/Game/GameContent/SavedData.SavedData_C|GetvoiceVol _assaved_data))
  (Development|PrintText (Utilities|Text|ToText(Float) (Variables|/Game/GameContent/SavedData.SavedData_C|GetvoiceVol _assaved_data) "HalfToEven")))