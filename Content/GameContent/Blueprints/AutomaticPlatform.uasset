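; AutomaticPlatform is a moving platform that shuttles between its starting position and an EndPoint component.
; BeginPlay caches both world locations and sets the timeline play rate from PlayRate.
; StartRoute and EndRoute overlaps with an AutomaticPlatform actor flip a Reverse flag, which Tick reads every frame to play or reverse the timeline.
; The timeline update lerps the Platform component between the two locations without sweep.
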(event OnComponentBeginOverlap(EndRoute)
  (params (OverlappedComponent :type Primitive%20Component%20Object%20Reference) (OtherActor :type Actor%20Object%20Reference) (OtherComp :type Primitive%20Component%20Object%20Reference) (OtherBodyIndex :type Integer) (bFromSweep :type Boolean) (SweepResult :type Hit%20Result%20Structure%20%28by%20ref%29))
  (Utilities|Casting|CastToAutomaticPlatform OtherActor)
  (Variables|Default|SetReverse true))

(event OnComponentBeginOverlap(StartRoute)
  (params (OverlappedComponent :type Primitive%20Component%20Object%20Reference) (OtherActor :type Actor%20Object%20Reference) (OtherComp :type Primitive%20Component%20Object%20Reference) (OtherBodyIndex :type Integer) (bFromSweep :type Boolean) (SweepResult :type Hit%20Result%20Structure%20%28by%20ref%29))
  (Utilities|Casting|CastToAutomaticPlatform OtherActor)
  (Variables|Default|SetReverse false))

(event EventTick
  (params (DeltaSeconds :type Float%20%28single-precision%29))
  (if (Variables|Default|GetReverse)
    (bind _newtrack_0 (Timeline|Timeline_0 Reverse)
      (:Update
        (Transformation|SetWorldLocation (Variables|Default|GetPlatform) (Math|Vector|Lerp(Vector) (Variables|Default|GetStartLoc) (Variables|Default|GetEndLoc) _newtrack_0) false false)))
    (else
      (Timeline|Timeline_0 Play))))

(event EventBeginPlay
  (Variables|Default|SetStartLoc (Transformation|GetWorldLocation (Variables|Default|GetPlatform)))
  (Variables|Default|SetEndLoc (Transformation|GetWorldLocation (Variables|Default|GetEndPoint)))
  (Components|Timeline|SetPlayRate (Variables|Default|GetTimeline_0) (Variables|Default|GetPlayRate)))

(fn ConstructionScript)

(fn SetLocations)