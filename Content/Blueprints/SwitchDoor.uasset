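; SwitchDoor is a door that slides between two positions when E is pressed inside its trigger.
; Overlapping PlayerTouch enables player 0's input and leaving disables it; the character cast runs afterward, so any actor triggers both.
; A FlipFlop alternately plays and reverses the DoorCntrol timeline, lerping Door from its starting location to DoorFinalPosition, both cached at BeginPlay, when PlayRate is also applied.
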(event OnComponentBeginOverlap(PlayerTouch)
  (params (OverlappedComponent :type Primitive%20Component%20Object%20Reference) (OtherActor :type Actor%20Object%20Reference) (OtherComp :type Primitive%20Component%20Object%20Reference) (OtherBodyIndex :type Integer) (bFromSweep :type Boolean) (SweepResult :type Hit%20Result%20Structure%20%28by%20ref%29))
  (Input|EnableInput (Game|GetPlayerController 0))
  (Utilities|Casting|CastToFirstPersonCharacter OtherActor))

(event OnComponentEndOverlap(PlayerTouch)
  (params (OverlappedComponent :type Primitive%20Component%20Object%20Reference) (OtherActor :type Actor%20Object%20Reference) (OtherComp :type Primitive%20Component%20Object%20Reference) (OtherBodyIndex :type Integer))
  (Input|DisableInput (Game|GetPlayerController 0))
  (Utilities|Casting|CastToFirstPersonCharacter OtherActor))

(event EventBeginPlay
  (Variables|Default|SetStartLoc (Transformation|GetWorldLocation (Variables|Default|GetDoor)))
  (Variables|Default|SetEndLoc (Transformation|GetWorldLocation (Variables|Default|GetDoorFinalPosition)))
  (Components|Timeline|SetPlayRate (Variables|Default|GetDoorCntrol) (Variables|Default|GetPlayRate)))

(event Input|KeyboardEvents|E
  (params (Key :type Key%20Structure))
  (:Pressed
    (Utilities|FlowControl|FlipFlop
      (:A
        (bind _doormovement (Timeline|DoorCntrol Play)
          (:Update
            (Transformation|SetWorldLocation (Variables|Default|GetDoor) (Math|Vector|Lerp(Vector) (Variables|Default|GetStartLoc) (Variables|Default|GetEndLoc) _doormovement) false false))))
      (:B
        (Timeline|DoorCntrol Reverse)))))

(fn ConstructionScript)

(fn SetLocations)