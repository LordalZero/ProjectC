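; Moving platform that travels between its starting position and an EndPoint component while the first-person character overlaps its PlayerTouch component.
; BeginPlay caches both world locations and applies PlayRate to the timeline.
; Overlap begin plays the timeline, which lerps the platform's location without sweep, and overlap end reverses it.
; The IsActive branch, construction script and SetLocations function are empty stubs.
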(event OnComponentBeginOverlap(PlayerTouch)
  (params (OverlappedComponent :type Primitive%20Component%20Object%20Reference) (OtherActor :type Actor%20Object%20Reference) (OtherComp :type Primitive%20Component%20Object%20Reference) (OtherBodyIndex :type Integer) (bFromSweep :type Boolean) (SweepResult :type Hit%20Result%20Structure%20%28by%20ref%29))
  (Utilities|Casting|CastToFirstPersonCharacter OtherActor)
  (bind _newtrack_0 (Timeline|Timeline_0 Play)
    (:Update
      (Transformation|SetWorldLocation (Variables|Default|GetPlatform) (Math|Vector|Lerp(Vector) (Variables|Default|GetStartLoc) (Variables|Default|GetEndLoc) _newtrack_0) false false))))

(event OnComponentEndOverlap(PlayerTouch)
  (params (OverlappedComponent :type Primitive%20Component%20Object%20Reference) (OtherActor :type Actor%20Object%20Reference) (OtherComp :type Primitive%20Component%20Object%20Reference) (OtherBodyIndex :type Integer))
  (Utilities|Casting|CastToFirstPersonCharacter OtherActor)
  (bind _newtrack_0 (Timeline|Timeline_0 Reverse)
    (:Update
      (Transformation|SetWorldLocation (Variables|Default|GetPlatform) (Math|Vector|Lerp(Vector) (Variables|Default|GetStartLoc) (Variables|Default|GetEndLoc) _newtrack_0) false false))))

(event EventBeginPlay
  (Variables|Default|SetStartLoc (Transformation|GetWorldLocation (Variables|Default|GetPlatform)))
  (Variables|Default|SetEndLoc (Transformation|GetWorldLocation (Variables|Default|GetEndPoint)))
  (Components|Timeline|SetPlayRate (Variables|Default|GetTimeline_0) (Variables|Default|GetPlayRate))
  (if (Variables|Default|GetIsActive)
    _))

(fn ConstructionScript)

(fn SetLocations)